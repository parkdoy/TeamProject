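; Game state for the shooting game that tracks the player list, spawns the magnetic field and shows state-driven player widgets.
; On BeginPlay, the authority caches the first player's controller and character, then spawns BP_MagneticField at a random navigable point around a fixed origin.
; ChangeGameState scans all shooting characters, creating PlayerIconWidget for ragdolled ones during Playing or End Game, and BP_WinWidget for the others at End Game.
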(event `AddPlayerToList`
  (params (Player :type "Character Object Reference"))
  ;[1 1 1] Add Player to List
  (`KismetArrayLibrary.Array_Add` (`self.PlayerList`) Player))

(event `SpawnMF(Client)`
  (`self.SpawnMF`))

(event `self.ReceiveBeginPlay`
  ;[1 1 1] 컨트롤러, 게임모드 초기화
  (`/Engine/EditorBlueprintResources/ActorMacros.Switch Has Authority`
    (:`Authority`
      (bind _asbp_shooting_player_controller (cast `/Game/ShootingGame/GameMode/BP_ShootingPlayerController` (`GameplayStatics.GetPlayerController` 0)))
      (set `self.PlayerController` _asbp_shooting_player_controller)
      (bind _asbp_shooting_character (cast `/Game/ShootingGame/GameMode/BP_ShootingCharacter` (`GameplayStatics.GetPlayerCharacter` 0)))
      (set `self.Character` _asbp_shooting_character)
      (`self.SpawnMF(Client)`))))

(event `ChangeGameState`
  (switch `/Game/ShootingGame/GameMode/EN-GameState` (`self.CurrentState`)
    (:`NewEnumerator0`
      (bind _outactors (`GameplayStatics.GetAllActorsOfClass` "/Game/ShootingGame/GameMode/BP_ShootingCharacter.BP_ShootingCharacter_C"))
      (for _array_element _outactors
        (if (`/Game/ShootingGame/GameMode/BP_ShootingCharacter.Ragdolled` _array_element)
          (bind _asbp_shooting_player_controller (cast `/Game/ShootingGame/GameMode/BP_ShootingPlayerController` (`Pawn.GetController` _array_element)))
          (bind _returnvalue (`|CreateWidget` "/Game/ShootingGame/Widget/PlayerIconWidget.PlayerIconWidget_C" _asbp_shooting_player_controller :!label _label))
          (`UserWidget.AddToViewport` _returnvalue 0))))
    (:`NewEnumerator1`
      (bind _outactors_2 (`GameplayStatics.GetAllActorsOfClass` "/Game/ShootingGame/GameMode/BP_ShootingCharacter.BP_ShootingCharacter_C"))
      (for _array_element_2 _outactors_2
        (if (`/Game/ShootingGame/GameMode/BP_ShootingCharacter.Ragdolled` _array_element_2)
          (goto _label)
          (else
            (bind _asbp_shooting_player_controller_2 (cast `/Game/ShootingGame/GameMode/BP_ShootingPlayerController` (`Pawn.GetController` _array_element_2)))
            (bind _returnvalue_2 (`|CreateWidget` "/Game/ShootingGame/Widget/BP_WinWidget.BP_WinWidget_C" _asbp_shooting_player_controller_2))
            (`UserWidget.AddToViewport` _returnvalue_2 0)))))))

(fn `OnRep_CurrentState`)

(fn `SpawnMF`
  (bind (_returnvalue_x _returnvalue_y _returnvalue_z) (`KismetMathLibrary.BreakVector` (`KismetMathLibrary.MakeVector` -600.0 -440.0 -40.0)))
  (bind _randomlocation (`NavigationSystemV1.K2_GetRandomLocationInNavigableRadius` (`KismetMathLibrary.MakeVector` _returnvalue_x _returnvalue_y) 10000.0 null null))
  (bind _returnvalue (`|SpawnActorFromClass` "/Game/ShootingGame/BattleRoyaleCircle/BP_MagneticField.BP_MagneticField_C" (`KismetMathLibrary.MakeTransform` (`KismetMathLibrary.MakeVector` (.x _randomlocation) (.y _randomlocation) _returnvalue_z)) "Undefined" "OverrideRootScale" null null))
  (set `self.MField` _returnvalue))

(fn `UserConstructionScript`)