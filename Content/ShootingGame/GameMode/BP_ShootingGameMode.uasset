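; Game mode for a shooting game that spawns characters for joining players, tracks live AI and drives match state.
; PostLogin has each shooting player controller spawn its character, then sets Survivor to the player count.
; AI count events adjust AIAlive, and a decrease below AIMax notifies the BP_AISpawner found in the level.
; BeginPlay caches and initializes the game state; CountSurvivor and OnlyOneLeft each set a state and call ChangeGameState.
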(event `IncreaseAI`
  ;[1 1 1] Control AINumvber
  (set `self.AI_Alive` (+ (`self.AI_Alive`) 1)))

(event `DecreaseAI`
  (bind _ai_alive (`self.AI_Alive`))
  ;[1 1 1] Control AINumvber
  (set `self.AI_Alive` (- _ai_alive 1))
  (if (< _ai_alive (`self.AI_Max`))
    (bind _returnvalue (`GameplayStatics.GetActorOfClass` "/Game/ShootingGame/AI/AI_Blueprint/BP_AISpawner.BP_AISpawner_C"))
    (`/Game/ShootingGame/AI/AI_Blueprint/BP_AISpawner.NoticeToGM` _returnvalue)))

(event `self.K2_PostLogin`
  (params (NewPlayer :type "PlayerController Object Reference"))
  (bind _asbp_shooting_player_controller (cast `/Game/ShootingGame/GameMode/BP_ShootingPlayerController` NewPlayer))
  (`/Game/ShootingGame/GameMode/BP_ShootingPlayerController.SpawnCharacter` _asbp_shooting_player_controller)
  (bind _returnvalue (`self.GetNumPlayers`))
  (set `self.Survivor` _returnvalue))

(event `self.ReceiveBeginPlay`
  (bind _asbp_shooting_game_state (cast `/Game/ShootingGame/GameMode/BP_ShootingGameState` (`GameplayStatics.GetGameState`)))
  (bind _output_get (set `self.GS_Ref` _asbp_shooting_game_state))
  (set `/Game/ShootingGame/GameMode/BP_ShootingGameState.CurrentState` "NewEnumerator2" _output_get))

(event `CountSurvivor`
  (bind _gs_ref (`self.GS_Ref`))
  (set `/Game/ShootingGame/GameMode/BP_ShootingGameState.CurrentState` "NewEnumerator0" _gs_ref)
  (`/Game/ShootingGame/GameMode/BP_ShootingGameState.ChangeGameState` _gs_ref))

(event `OnlyOneLeft`
  (bind _gs_ref (`self.GS_Ref`))
  (set `/Game/ShootingGame/GameMode/BP_ShootingGameState.CurrentState` "NewEnumerator1" _gs_ref)
  (`/Game/ShootingGame/GameMode/BP_ShootingGameState.ChangeGameState` _gs_ref))

(fn `UserConstructionScript`)