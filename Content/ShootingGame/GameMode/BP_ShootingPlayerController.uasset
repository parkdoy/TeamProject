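; Player controller for the shooting game that spawns the player's selected character and applies their name.
; On possession, it reads the name from ShootingGameInstance and passes it through client-response and request events to the player state.
; SpawnCharacter passes the selected class to SpawnCharacterServer, which claims an unused PlayerStart by tagging it "Found", then spawns and possesses the character there.
; BeginPlay sets game-only input.
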(event `self.ReceivePossess`
  (params (PossessedPawn :type "Pawn Object Reference"))
  (`self.ResClientPossess`))

(event `ResClientPossess`
  (bind _asshooting_game_instance (cast `/Game/ShootingGame/GameMode/ShootingGameInstance` (`GameplayStatics.GetGameInstance`)))
  (`self.ReqSetName` (`/Game/ShootingGame/GameMode/ShootingGameInstance.Name` _asshooting_game_instance)))

(event `ReqSetName`
  (params (NewName :type String))
  (bind _asbp_shooting_player_state (cast `/Game/ShootingGame/GameMode/BP_ShootingPlayerState` (`self.PlayerState`)))
  (`/Game/ShootingGame/GameMode/BP_ShootingPlayerState.SetName` _asbp_shooting_player_state NewName))

(event `self.ReceiveBeginPlay`
  (`WidgetBlueprintLibrary.SetInputMode_GameOnly` self))

(event `SpawnCharacter`
  (bind _asshooting_game_instance (cast `/Game/ShootingGame/GameMode/ShootingGameInstance` (`GameplayStatics.GetGameInstance`)))
  (`self.SpawnCharacterServer` (`/Game/ShootingGame/GameMode/ShootingGameInstance.SelectedCharacter` _asshooting_game_instance)))

(event `SpawnCharacterServer`
  (params (Class :type "Character Class Reference"))
  (bind _outactors (`GameplayStatics.GetAllActorsOfClass` "/Script/Engine.PlayerStart"))
  (for _array_element _outactors
    (if (!= (`PlayerStart.PlayerStartTag` _array_element) "Found")
      (set `PlayerStart.PlayerStartTag` "Found" _array_element)
      (break)))
  (bind _returnvalue (`|SpawnActorFromClass` Class (`self.GetTransform` _array_element) "Undefined" "OverrideRootScale" null null))
  (`self.Possess` self _returnvalue))

(fn `UserConstructionScript`)