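; BP_AI_Wolf is a wolf AI enemy for the shooting game that takes weapon damage and dies.
; A sphere overlap shows or hides its world health widget when the player character enters or leaves, and BeginPlay links that widget to the wolf.
; Only damage caused by BP_Weapon lowers HP.
; At zero HP, a DoOnce triggers death: it detaches the controller, plays a death montage, then spawns an item after a short delay.
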(event `self.ReceiveBeginPlay`
  (`parent.ReceiveBeginPlay`)
  (bind _asbp_shooting_game_mode (cast `/Game/ShootingGame/GameMode/BP_ShootingGameMode` (`GameplayStatics.GetGameMode`)))
  (set `self.ShootingGM_REF` _asbp_shooting_game_mode)
  (bind _asaihealth_widget (cast `/Game/ShootingGame/AI/AI_Widget/AIHealthWidget` (`WidgetComponent.GetUserWidgetObject` (`self.AIHealthWidget`))))
  (bind _output_get (set `self.AIHealth_Widget` _asaihealth_widget))
  (set `/Game/ShootingGame/AI/AI_Widget/AIHealthWidget.AI` self _output_get))

(event `self.Sphere.OnComponentBeginOverlap`
  (params (OverlappedComponent :type "PrimitiveComponent Object Reference") (OtherActor :type "Actor Object Reference") (OtherComp :type "PrimitiveComponent Object Reference") (OtherBodyIndex :type Integer) (bFromSweep :type Boolean) (SweepResult :type "HitResult Structure (by ref)"))
  (cast `/Game/ShootingGame/GameMode/BP_ShootingCharacter` OtherActor)
  (`SceneComponent.SetVisibility` (`self.AIHealthWidget`) true false))

(event `self.Sphere.OnComponentEndOverlap`
  (params (OverlappedComponent :type "PrimitiveComponent Object Reference") (OtherActor :type "Actor Object Reference") (OtherComp :type "PrimitiveComponent Object Reference") (OtherBodyIndex :type Integer))
  (cast `/Game/ShootingGame/GameMode/BP_ShootingCharacter` OtherActor)
  (`SceneComponent.SetVisibility` (`self.AIHealthWidget`) false false))

(event `self.ReceiveAnyDamage`
  (params (Damage :type "Float (single-precision)") (DamageType :type "DamageType Object Reference") (InstigatedBy :type "Controller Object Reference") (DamageCauser :type "Actor Object Reference"))
  (cast `/Game/ShootingGame/Blueprint/BP_Weapon` DamageCauser)
  (bind _output_get (set `self.HP` (- (`self.HP`) Damage)))
  (if (<= _output_get 0.0)
    (`/Engine/EditorBlueprintResources/StandardMacros.DoOnce` false
      (:`Completed`
        (`self.ResWolfDeath`)))))

(event `ResWolfDeath`
  (`self.Death`)
  (`KismetSystemLibrary.Delay` 2.0)
  (`self.SpawnItem`))

(fn `Death`
  (`self.DetachFromControllerPendingDestroy`)
  (`self.PlayAnimMontage` "/Game/AnimalVarietyPack/Wolf/Animations/ANIM_Wolf_Death_Montage.ANIM_Wolf_Death_Montage"))

(fn `UserConstructionScript`
  (`parent.UserConstructionScript`))