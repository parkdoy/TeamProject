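; BP_SpawnItem is an item spawn point that places one random item from its Items array at its own transform.
; BeginPlay calls SpawnItem, which spawns only with authority and adjusts for collision but always spawns.
; Respawn logic is unwired: the OnDestroyed binding and DestroyItem's timer back to SpawnItem never run, so nothing replaces a destroyed item.
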(event `self.ReceiveBeginPlay`
  (`self.SpawnItem`))

(fn `DestroyItem`
  (params (DestroyedActor :type "Actor Object Reference")))

(fn `SpawnItem`
  (`/Engine/EditorBlueprintResources/ActorMacros.Switch Has Authority`
    (:`Authority`
      (`|SpawnActorFromClass` (`KismetArrayLibrary.Array_Random` (`self.Items`)) (`self.GetTransform`) "AdjustIfPossibleButAlwaysSpawn" "OverrideRootScale" null null))))

(fn `UserConstructionScript`)