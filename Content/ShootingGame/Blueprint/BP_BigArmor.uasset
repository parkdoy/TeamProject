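; BP_BigArmor is an armor pickup item for the shooting game that grants a large fixed amount of armor.
; It spins by adding a small rotation to its root component every tick.
; Its UseItem override calls the parent check, then on success adds armor through the character's BP_ShootingPlayerState and destroys itself.
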(event `self.ReceiveTick`
  (params (DeltaSeconds :type "Float (single-precision)"))
  (`SceneComponent.K2_AddRelativeRotation` (`self.DefaultSceneRoot`) (struct :`Yaw` 2.5) false false))

(fn `UseItem`
  (params (Character :type "Character Object Reference"))
  (bind _isuse (`parent.UseItem` Character))
  (if _isuse
    (bind _asbp_shooting_player_state (cast `/Game/ShootingGame/GameMode/BP_ShootingPlayerState` (`Pawn.PlayerState` Character)))
    (`/Game/ShootingGame/GameMode/BP_ShootingPlayerState.AddArmor` _asbp_shooting_player_state 60.0)
    (`self.K2_DestroyActor`)))

(fn `UserConstructionScript`
  (`parent.UserConstructionScript`))