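; BP_Item is a pickup item for the shooting game that spins in place and checks characters that touch it.
; Tick rotates the StaticMesh by a fixed step each frame, and its begin-overlap event passes any Character to UseItem.
; UseItem returns true only on authority for a living BP_ShootingCharacter.
; It applies no effect itself, and the overlap event ignores the result.
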(event `self.ReceiveTick`
  (params (DeltaSeconds :type "Float (single-precision)"))
  (`SceneComponent.K2_AddRelativeRotation` (`self.StaticMesh`) (struct :`Yaw` 2.5) false false))

(event `self.StaticMesh.OnComponentBeginOverlap`
  (params (OverlappedComponent :type "PrimitiveComponent Object Reference") (OtherActor :type "Actor Object Reference") (OtherComp :type "PrimitiveComponent Object Reference") (OtherBodyIndex :type Integer) (bFromSweep :type Boolean) (SweepResult :type "HitResult Structure (by ref)"))
  (bind _ascharacter (cast `Character` OtherActor))
  (`self.UseItem` _ascharacter))

(fn `UseItem`
  (params (Character :type "Character Object Reference"))
  (returns (IsUse :type Boolean))
  (`/Engine/EditorBlueprintResources/ActorMacros.Switch Has Authority`
    (:`Authority`
      (bind _asbp_shooting_character (cast `/Game/ShootingGame/GameMode/BP_ShootingCharacter` Character))
      (if (`/Game/ShootingGame/GameMode/BP_ShootingCharacter.IsDie` _asbp_shooting_character)
        (return false)
        (else
          (return true))))
    (:`Remote`
      (return false))))

(fn `UserConstructionScript`)